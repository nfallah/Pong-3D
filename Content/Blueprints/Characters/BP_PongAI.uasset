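; BP_PongAI is a Pong opponent that moves along a fixed line to follow the ball projectile's X position.
; After a delay on BeginPlay, a custom event issues AIMoveTo toward that X, clamped to the court range, with fixed Y and Z.
; The event re-calls itself on success or failure, forming a continuous chase loop.
; Its debug prints are swapped between outcomes, and the AIUpdate event is empty.
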(event `self.ReceiveBeginPlay`
  (`KismetSystemLibrary.Delay` 6.0)
  (`self.poopy`))

(event `/Game/Blueprints/Interfaces/BPI_UpdateAIMovement.AI Update`
  (params (`BP Projectile` :type "/Game/Blueprints/Characters/BP_Projectile Object Reference")))

(event `poopy`
  (bind _returnvalue_x (`KismetMathLibrary.BreakVector` (`self.K2_GetActorLocation` (stale `/Game/Blueprints/Interfaces/BPI_UpdateAIMovement.AI Update` `BP Projectile`))))
  (`|AIMoveTo` self (`KismetMathLibrary.MakeVector` (`KismetMathLibrary.FClamp` _returnvalue_x -400.0 400.0) 950.0 35.0) null
    (:`OnSuccess`
      (`KismetSystemLibrary.PrintString` "FAILED" true true (struct :`R` 1.0 :`A` 1.0)))
    (:`OnFail`
      (`KismetSystemLibrary.PrintString` "FINISHED" true true (struct :`G` 1.0 :`A` 1.0))))
  (`self.poopy`))

(fn `UserConstructionScript`)