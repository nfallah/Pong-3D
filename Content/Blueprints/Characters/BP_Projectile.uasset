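; BP_Projectile is a projectile that, once started, launches in the XY plane after a short delay and keeps its speed bounded.
; StartProjectile calls GenerateProjectileVelocity, which randomizes the sign of each axis, and applies its velocity output when the delay ends.
; Tick then records the current X and Y direction signs and clamps each component between per-axis minimums and a shared maximum, preserving direction.
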(event `/Game/Blueprints/Interfaces/BPI_StartProjectile.StartProjectile`
  (`|ExecutionSequence`
    (:`then_0`
      (`KismetSystemLibrary.Delay` 1.5)
      (set `MovementComponent.Velocity` (`KismetMathLibrary.MakeVector` (stale _velocity_x) (stale _velocity_y)) (`self.Projectile Movement`))
      (set `self.Check For Movement?` true))
    (:`then_1`
      (bind (_velocity_x _velocity_y) (`self.Generate Projectile Velocity`)))))

(event `self.ReceiveTick`
  (params (DeltaSeconds :type "Float (single-precision)"))
  (if (`self.Check For Movement?`)
    (`self.Calculate Current Direction`)
    (`self.Clamp Velocity Based On Direction`)))

(fn `Calculate Current Direction`
  (bind (_velocity_x _velocity_y) (`KismetMathLibrary.BreakVector` (`MovementComponent.Velocity` (`self.Projectile Movement`))))
  (`|ExecutionSequence`
    (:`then_0`
      (`/Engine/EditorBlueprintResources/StandardMacros.CompareFloat` _velocity_x
        (:`>`
          (set `self.Current Velocity Direction in X` 1))
        (:`<`
          (set `self.Current Velocity Direction in X` -1))))
    (:`then_1`
      (`/Engine/EditorBlueprintResources/StandardMacros.CompareFloat` _velocity_y
        (:`>`
          (set `self.Current Velocity Direction in Y` 1))
        (:`<`
          (set `self.Current Velocity Direction in Y` -1))))))

(fn `Clamp Velocity Based On Direction`
  (bind (_velocity_x _velocity_y _velocity_z) (`KismetMathLibrary.BreakVector` (`MovementComponent.Velocity` (`self.Projectile Movement`))))
  (bind (_velocity_x_2 _velocity_y_2 _velocity_z_2) (`KismetMathLibrary.BreakVector` (`MovementComponent.Velocity` (`self.Projectile Movement`))))
  (bind (_velocity_x_3 _velocity_y_3 _velocity_z_3) (`KismetMathLibrary.BreakVector` (`MovementComponent.Velocity` (`self.Projectile Movement`))))
  (bind (_velocity_x_4 _velocity_y_4 _velocity_z_4) (`KismetMathLibrary.BreakVector` (`MovementComponent.Velocity` (`self.Projectile Movement`))))
  (`|ExecutionSequence`
    (:`then_0`
      (`/Engine/EditorBlueprintResources/StandardMacros.CompareInt` (`self.Current Velocity Direction in X`)
        (:`>`
          (set `MovementComponent.Velocity` (`KismetMathLibrary.MakeVector` (`KismetMathLibrary.FClamp` _velocity_x (`self.Minimum Speed X`) (`self.Maximum Speed X and Y`)) _velocity_y _velocity_z) (`self.Projectile Movement`)))
        (:`<`
          (set `MovementComponent.Velocity` (`KismetMathLibrary.MakeVector` (`KismetMathLibrary.FClamp` _velocity_x_2 (* (`self.Current Velocity Direction in X`) (`self.Maximum Speed X and Y`)) (* (`self.Current Velocity Direction in X`) (`self.Minimum Speed X`))) _velocity_y_2 _velocity_z_2) (`self.Projectile Movement`)))))
    (:`then_1`
      (`/Engine/EditorBlueprintResources/StandardMacros.CompareInt` (`self.Current Velocity Direction in Y`)
        (:`>`
          (set `MovementComponent.Velocity` (`KismetMathLibrary.MakeVector` _velocity_x_4 (`KismetMathLibrary.FClamp` _velocity_y_4 (`self.Minimum Speed Y`) (`self.Maximum Speed X and Y`)) _velocity_z_4) (`self.Projectile Movement`)))
        (:`<`
          (set `MovementComponent.Velocity` (`KismetMathLibrary.MakeVector` _velocity_x_3 (`KismetMathLibrary.FClamp` _velocity_y_3 (* (`self.Current Velocity Direction in Y`) (`self.Maximum Speed X and Y`)) (* (`self.Current Velocity Direction in Y`) (`self.Minimum Speed Y`))) _velocity_z_3) (`self.Projectile Movement`)))))))

(fn `UserConstructionScript`)